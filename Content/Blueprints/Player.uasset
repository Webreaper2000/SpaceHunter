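; Player Blueprint whose only active logic toggles the pause menu with the M key.
; When unpaused, M shows the cursor, switches to Game and UI input focused on the menu, adds it to the viewport and pauses the game.
; The Pausemenu widget is created on first use and cached in PauseMenuReference.
; When paused, M hides the cursor, restores game-only input, removes the menu and unpauses.
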(event `self.ReceiveBeginPlay`)

(event `Key|M` :paused true
  (params (Key :type "Key Structure" :default "AnyKey"))
  (bind _returnvalue (`GameplayStatics.GetPlayerController` 0))
  (bind _pause_menu_reference (`self.Pause menu reference`))
  (:`Pressed`
    (if (`GameplayStatics.IsGamePaused`)
      (set `PlayerController.bShowMouseCursor` false _returnvalue)
      (`WidgetBlueprintLibrary.SetInputMode_GameOnly` _returnvalue)
      (`Widget.RemoveFromParent` _pause_menu_reference)
      (`GameplayStatics.SetGamePaused` false)
      (else
        (set `PlayerController.bShowMouseCursor` true _returnvalue)
        (`/Engine/EditorBlueprintResources/StandardMacros.IsValid` _pause_menu_reference
          (:`Is Valid`
            _)
          (:`Is Not Valid`
            (bind _returnvalue_2 (`|CreateWidget` "/Game/Blueprints/Pausemenu.Pausemenu_C"))
            (set `self.Pause menu reference` _returnvalue_2)))
        (`WidgetBlueprintLibrary.SetInputMode_GameAndUIEx` _returnvalue _pause_menu_reference)
        (`UserWidget.AddToViewport` _pause_menu_reference 0)
        (`GameplayStatics.SetGamePaused` true)))))

(fn `UserConstructionScript`)